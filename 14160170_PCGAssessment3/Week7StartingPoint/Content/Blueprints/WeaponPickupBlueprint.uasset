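; Weapon pickup actor that passes its stats to the gun of the actor that picks it up.
; BeginPlay calls OnGenerate, then loops over every rarity enum value, applying each matching gold, purple, blue or white material in turn rather than checking one rolled rarity.
; OnPickup finds the picker's child-actor GunBlueprint, copies magazine, velocity, damage and accuracy values, refills the magazine and destroys the pickup.
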(event `self.ReceiveBeginPlay`
  (bind _skeletalmesh (`self.SkeletalMesh`))
  (`self.OnGenerate`)
  (bind _enumvalue (foreach `EWeaponPickupRarity` false)
    (:`LoopBody`
      (if (`|EnumEquality` "LEGENDARY" _enumvalue)
        (bind _returnvalue (`PrimitiveComponent.CreateDynamicMaterialInstance` _skeletalmesh 0 "/Game/Materials/Gun_Gold_Inst.Gun_Gold_Inst" "None"))
        (`MaterialInstanceDynamic.SetVectorParameterValue` :`self` _returnvalue)
        (elif (`|EnumEquality` "MASTER" _enumvalue)
          (`PrimitiveComponent.CreateDynamicMaterialInstance` _skeletalmesh 0 "/Game/Materials/Gun_Purple_Inst.Gun_Purple_Inst" "None")
          (elif (`|EnumEquality` "RARE" _enumvalue)
            (`PrimitiveComponent.CreateDynamicMaterialInstance` _skeletalmesh 0 "/Game/Materials/Gun_Blue_Inst.Gun_Blue_Inst" "None")
            (elif (`|EnumEquality` "COMMON" _enumvalue)
              (`PrimitiveComponent.CreateDynamicMaterialInstance` _skeletalmesh 0 "/Game/Materials/Gun_White_Inst.Gun_White_Inst" "None"))))))))

(event `self.OnPickup`
  (params (ActorThatPickedUp :type "Actor Object Reference"))
  (bind _magazinesize (`self.MagazineSize`))
  (bind _asgun_blueprint (cast `/Game/Blueprints/GunBlueprint` (`ChildActorComponent.ChildActor` (`self.GetComponentByClass` ActorThatPickedUp "/Script/Engine.ChildActorComponent"))))
  (set `/Game/Blueprints/GunBlueprint.MagazineSize` _magazinesize _asgun_blueprint)
  (set `/Game/Blueprints/GunBlueprint.RoundsRemainingInMagazine` _magazinesize _asgun_blueprint)
  (set `/Game/Blueprints/GunBlueprint.MuzzleVelocity` (`self.MuzzleVelocity`) _asgun_blueprint)
  (set `/Game/Blueprints/GunBlueprint.BulletDamage` (`self.BulletDamage`) _asgun_blueprint)
  (set `/Game/Blueprints/GunBlueprint.WeaponAccuracy` (`self.WeaponAccuracy`) _asgun_blueprint)
  (`self.K2_DestroyActor`))

(fn `UserConstructionScript`)